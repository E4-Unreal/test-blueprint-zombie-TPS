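; BP_DroppedItem is a pickup actor that shows an item info widget when the player is nearby and looking at it.
; Overlap with the player enables a per-tick camera-forward sphere trace against only its static mesh, toggling the widget and registering the item as the character's LookingItem.
; Leaving range or looking away hides the widget and clears that reference.
; PickupItem copies ItemInfo to the character's LookingItemInfo, then destroys the actor.
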(event `self.ReceiveBeginPlay`
  (`SceneComponent.SetVisibility` (`self.ItemInfo_Widget`) false false)
  (bind _asui_item_info (cast `/Game/E4/HUD/UI_ItemInfo` (`WidgetComponent.GetUserWidgetObject` (`self.ItemInfo_Widget`))))
  (set `/Game/E4/HUD/UI_ItemInfo.Name` (`.Name_13_6936896D4C6D2F2BF77C41A755F61CA0` (break `/Game/E4/HUD/ItemStruct` (`self.ItemInfo`))) _asui_item_info)
  (bind _asbp_player_character (cast `/Game/E4/Blueprints/BP_PlayerCharacter` (`GameplayStatics.GetPlayerCharacter` 0)))
  (set `self.BP_PlayerCharacter` _asbp_player_character))

(event `self.ReceiveActorBeginOverlap`
  (params (OtherActor :type "Actor Object Reference"))
  (if (== OtherActor (`self.BP_PlayerCharacter`))
    (set `self.IsInRange` true)))

(event `self.ReceiveActorEndOverlap`
  (params (OtherActor :type "Actor Object Reference"))
  (if (== OtherActor (`self.BP_PlayerCharacter`))
    (set `self.IsInRange` false)
    (`self.Reset`)))

(event `self.ReceiveTick`
  (params (DeltaSeconds :type "Float (single-precision)"))
  (if (`self.IsInRange`)
    (`self.DisplayWidgetByLooking`)))

(event `/Game/E4/Blueprints/BP_Interface_Character.PickupItem`
  (set `/Game/E4/Blueprints/BP_PlayerCharacter.LookingItemInfo` (`self.ItemInfo`) (`self.BP_PlayerCharacter`))
  (`self.K2_DestroyActor`))

(fn `DisplayWidgetByLooking`
  (bind _returnvalue (`GameplayStatics.GetPlayerCameraManager` 0))
  (bind _returnvalue_2 (`PlayerCameraManager.GetCameraLocation` _returnvalue))
  (bind (_hitlocation _hitnormal _bonename _outhit _returnvalue_3) (`PrimitiveComponent.K2_SphereTraceComponent` (`self.StaticMesh`) _returnvalue_2 (+ _returnvalue_2 (* (`KismetMathLibrary.GetForwardVector` (`PlayerCameraManager.GetCameraRotation` _returnvalue)) 1500.0)) 40.0 true false false))
  (bind _output_get (set `self.IsLooking` _returnvalue_3))
  (if _output_get
    (`SceneComponent.SetVisibility` (`self.ItemInfo_Widget`) true false)
    (set `/Game/E4/Blueprints/BP_PlayerCharacter.LookingItem` self (`self.BP_PlayerCharacter`))
    (else
      (`self.Reset`))))

(fn `Reset`
  (`SceneComponent.SetVisibility` (`self.ItemInfo_Widget`) false false)
  (if (== (`/Game/E4/Blueprints/BP_PlayerCharacter.LookingItem` (`self.BP_PlayerCharacter`)) self)
    (set `/Game/E4/Blueprints/BP_PlayerCharacter.LookingItem` null (`self.BP_PlayerCharacter`))))

(fn `UserConstructionScript`)