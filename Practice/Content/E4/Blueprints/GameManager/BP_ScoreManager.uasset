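; Score manager that keeps a per-instigator scoreboard of kills, damage, attack count and headshots.
; RecordDeathInfo adds each death info entry to that instigator's RecordBoard struct, counting one kill per entry.
; SearchPlayer finds the instigator's index by linear search, appending a new record when none exists.
; Entries from the first player controller fire the PlayerKill dispatcher, which BeginPlay binds after casting the player character.
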(event `self.ReceiveBeginPlay`
  (bind _asbp_player_character (cast `/Game/E4/Blueprints/BP_PlayerCharacter` (`GameplayStatics.GetPlayerCharacter` 0)))
  (add `self.PlayerKill` (`|CreateDelegate` _asbp_player_character :!event `ShowKillLog`)))

(fn `RecordDeathInfo`
  (params (DeathInfo :type "Array of DeathInfoStruct Structure"))
  (for _array_element DeathInfo
    (bind (_instigator _killedclass _damage _attackcount _headshot) (break `DeathInfoStruct` _array_element))
    (bind _index (`self.SearchPlayer` _instigator))
    (bind _output (`|GetArrayItem` (`self.RecordBoard`) _index))
    (bind (_instigator_2 _killcount _damage_2 _attackcount_2 _headshot_2) (break `PlayRecordStruct` _output))
    (bind _structout (setmembers `PlayRecordStruct` :`StructRef` _output :`KillCount` (+ _killcount 1) :`Damage` (+ _damage _damage_2) :`AttackCount` (+ _attackcount _attackcount_2) :`HeadShot` (+ _headshot _headshot_2)))
    (`KismetArrayLibrary.Array_Set` (`self.RecordBoard`) _index _structout)
    (if (== _instigator (`GameplayStatics.GetPlayerController` 0))
      (`self.PlayerKill`))))

(fn `SearchPlayer`
  (params (Instigator :type "Controller Object Reference"))
  (returns (Index :type Integer))
  (for (_array_element _array_index) (`self.RecordBoard`)
    (if (== (`.Instigator` (break `PlayRecordStruct` _array_element)) Instigator)
      (return _array_index)))
  (bind _returnvalue (`KismetArrayLibrary.Array_Add` (`self.RecordBoard`) (make `PlayRecordStruct` Instigator)))
  (return _returnvalue))

(fn `UserConstructionScript`)