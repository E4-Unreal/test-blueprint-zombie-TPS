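; BP_GunWeapon is a gun weapon Blueprint that handles the ammo side of reloading.
; WantReload reports whether the gun is below its maximum bullet count, along with the bullet name and the number of bullets needed to fill it.
; The DoReload event adds the supplied bullets to the current count without clamping to the maximum.
; BeginPlay, overlap and Tick are disabled stubs, and the graphs contain no firing logic.
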(event `/Game/E4/Blueprints/Interface_PlayerToGunWeapon.DoReload`
  (params (ReloadingBullets :type Integer))
  (set `self.Bullets` (+ (`self.Bullets`) ReloadingBullets)))

(fn `UserConstructionScript`
  (`parent.UserConstructionScript`))

(fn `WantReload`
  (returns (CanReload :type Boolean) (BulletName :type Name) (NeedBullets :type Integer))
  (bind _maxbullets (`self.MaxBullets`))
  (bind _bullets (`self.Bullets`))
  (return (> _maxbullets _bullets) (`self.BulletName`) (- _maxbullets _bullets)))