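; BP_Knuckle is a melee weapon that damages the player on contact while active.
; Its Sphere collider starts with no collision, and UseItem arms it by switching to the CustomWeapon profile.
; When the sphere overlaps the player pawn, it applies fixed point damage using the sweep result and disables its collision, limiting each use to one hit.
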(event `self.ReceiveBeginPlay`
  (`PrimitiveComponent.SetCollisionProfileName` (`self.Sphere`) "NoCollision" true))

(event `self.Sphere.OnComponentBeginOverlap`
  (params (OverlappedComponent :type "PrimitiveComponent Object Reference") (OtherActor :type "Actor Object Reference") (OtherComp :type "PrimitiveComponent Object Reference") (OtherBodyIndex :type Integer) (bFromSweep :type Boolean) (SweepResult :type "HitResult Structure (by ref)"))
  (bind _returnvalue (`GameplayStatics.GetPlayerPawn` 0))
  (if (== OtherActor _returnvalue)
    (`GameplayStatics.ApplyPointDamage` _returnvalue 20.0 (`.ImpactPoint` (`GameplayStatics.BreakHitResult` SweepResult)) SweepResult)
    (`PrimitiveComponent.SetCollisionProfileName` (`self.Sphere`) "NoCollision" true)))

(event `/Game/E4/Blueprints/Interface_CharacterToItem.UseItem`
  (`PrimitiveComponent.SetCollisionProfileName` (`self.Sphere`) "CustomWeapon" true))

(fn `UserConstructionScript`)