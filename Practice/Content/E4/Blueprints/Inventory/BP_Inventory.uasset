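; BP_Inventory is a slot-based inventory actor that stores, stacks, withdraws and counts items by name.
; Its construction script creates SlotNum slots, and an item named "None" marks an empty one.
; AddNewItem tops up matching stacks to MaxCount and puts any remainder in the first free slot.
; GetItem drains matching stacks up to the requested count, clearing emptied slots and succeeding even when stock falls short.
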(event `self.ReceiveBeginPlay`)

(fn `Add`
  (params (NewItem :type "ItemStruct Structure"))
  (returns (IsSucceed :type Boolean))
  (for (_array_element _array_index) (`self.Inventory`)
    (if (== (`.Name` (break `ItemStruct` _array_element)) "None")
      (`KismetArrayLibrary.Array_Set` (`self.Inventory`) _array_index (`local.NewItem`))
      (return true))))

(fn `AddNewItem`
  (params (NewItem :type "ItemStruct Structure"))
  (returns (IsSucceed :type Boolean) (Count :type Integer))
  (locals (BufferCount :type Integer) (Items :type "Array of ItemStruct Structure") (Indices :type "Array of Integer"))
  (bind (_name _droppedclass _spawnedclass _spawnedactor _canequip _equiptype _count) (break `ItemStruct` NewItem))
  (bind (_isfind _items _indices) (`self.SearchItems` _name))
  (if _isfind
    (set `local.BufferCount` _count)
    (set `local.Items` _items)
    (set `local.Indices` _indices)
    (for (_array_element _array_index) (`local.Items`)
      (bind (_name_2 _droppedclass_2 _spawnedclass_2 _spawnedactor_2 _canequip_2 _equiptype_2 _count_2 _maxcount) (break `ItemStruct` _array_element))
      (bind _returnvalue (- _maxcount _count_2))
      (if (>= _returnvalue (`local.BufferCount`))
        (bind _structout (setmembers `ItemStruct` :`StructRef` _array_element :`Count` (+ _count_2 (`local.BufferCount`))))
        (`self.Set` (`|GetArrayItem` (`local.Indices`) _array_index) _structout)
        (set `local.BufferCount` 0)
        (return true 0)
        (else
          (set `local.BufferCount` (- (`local.BufferCount`) _returnvalue))
          (bind _structout_2 (setmembers `ItemStruct` :`StructRef` _array_element :`Count` _maxcount))
          (`self.Set` (`|GetArrayItem` (`local.Indices`) _array_index) _structout_2))))
    (if (> (`local.BufferCount`) 0)
      (bind _structout_3 (setmembers `ItemStruct` :`StructRef` (`|GetArrayItem` (`local.Items`)) :`Count` (`local.BufferCount`)))
      (bind _issucceed (`self.Add` _structout_3))
      (return _issucceed (`local.BufferCount`)))
    (else
      (bind _issucceed_2 (`self.Add` (`local.NewItem`)))
      (return _issucceed_2 0))))

(fn `GetItem`
  (params (ItemName :type Name) (NeedCount :type Integer))
  (returns (IsSucceed :type Boolean) (Item :type "ItemStruct Structure"))
  (locals (Indices :type "Array of Integer") (Items :type "Array of ItemStruct Structure") (OutputCount :type Integer) (BufferCount :type Integer))
  (bind _isfound (`self.SearchItem` ItemName))
  (if _isfound
    (bind (_isfind _items _indices) (`self.SearchItems` (`local.ItemName`)))
    (set `local.Items` _items)
    (set `local.Indices` _indices)
    (for (_array_element _array_index) (`local.Items`)
      (bind _output_get (set `local.BufferCount` (- (`local.NeedCount`) (`local.OutputCount`))))
      (bind (_name _droppedclass _spawnedclass _spawnedactor _canequip _equiptype _count) (break `ItemStruct` _array_element))
      (if (> _count _output_get)
        (set `local.OutputCount` (`local.NeedCount`))
        (bind _structout (setmembers `ItemStruct` :`StructRef` _array_element :`Count` (- _count (`local.BufferCount`))))
        (`self.Set` (`|GetArrayItem` (`local.Indices`) _array_index) _structout)
        (bind _structout_2 (setmembers `ItemStruct` :`StructRef` (`|GetArrayItem` (`local.Items`)) :`Count` (`local.OutputCount`) :!label _label))
        (return true _structout_2)
        (else
          (set `local.OutputCount` (+ (`local.OutputCount`) _count))
          (`self.Remove` (`|GetArrayItem` (`local.Indices`) _array_index)))))
    (goto _label)
    (else
      (return false))))

(fn `Remove`
  (params (Index :type Integer))
  (`KismetArrayLibrary.Array_Set` (`self.Inventory`) Index (make `ItemStruct` "None")))

(fn `SearchItem`
  (params (ItemName :type Name))
  (returns (IsFound :type Boolean))
  (for _array_element (`self.Inventory`)
    (if (== (`.Name` (break `ItemStruct` _array_element)) ItemName)
      (return true)))
  (return false))

(fn `SearchItemCount`
  (params (ItemName :type Name))
  (returns (TatalCount :type Integer))
  (locals (TotalCount :type Integer))
  (bind _isfound (`self.SearchItem` ItemName))
  (if _isfound
    (bind (_isfind _items) (`self.SearchItems` ItemName))
    (for _array_element _items
      (set `local.TotalCount` (+ (`.Count` (break `ItemStruct` _array_element)) (`local.TotalCount`))))
    (return (`local.TotalCount`))))

(fn `SearchItems`
  (params (Name :type Name))
  (returns (IsFind :type Boolean) (Items :type "Array of ItemStruct Structure") (Indices :type "Array of Integer"))
  (locals (ItemBuffer :type "Array of ItemStruct Structure") (IndexBuffer :type "Array of Integer"))
  (for (_array_element _array_index) (`self.Inventory`)
    (if (== (`.Name` (break `ItemStruct` _array_element)) (`local.Name`))
      (`KismetArrayLibrary.Array_Add` (`local.ItemBuffer`) _array_element)
      (`KismetArrayLibrary.Array_Add` (`local.IndexBuffer`) _array_index)))
  (if (> (`KismetArrayLibrary.Array_Length` (`local.ItemBuffer`)) 0)
    (return true (`local.ItemBuffer`) (`local.IndexBuffer`))
    (else
      (return false))))

(fn `Set`
  (params (Index :type Integer) (Item :type "ItemStruct Structure"))
  (if (<= (`.Count` (break `ItemStruct` Item)) 0)
    (`self.Remove` Index)
    (else
      (`KismetArrayLibrary.Array_Set` (`self.Inventory`) Index Item))))

(fn `UserConstructionScript`
  (for _ (range 1 (+ (`self.SlotNum`) 1))
    (`KismetArrayLibrary.Array_Add` (`self.Inventory`))))