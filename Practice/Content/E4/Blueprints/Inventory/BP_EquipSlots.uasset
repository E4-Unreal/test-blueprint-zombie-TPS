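; Equipment slot manager actor owned by the player character, holding weapon and gear items in one array sized at construction, weapons first.
; AddNewEquip finds an empty slot by type, though the gear search ends at EquipNum-1 rather than offsetting by WeaponNum.
; AddEquip spawns the item actor, attaching it to the slot's character mesh socket or disabling it if none.
; WeaponCursor selects the active weapon; setting it calls the character's GetPrimaryWeapon.
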(fn `AddEquip`
  (params (EquipInfo :type "ItemStruct Structure") (Cursor :type Integer))
  (bind _returnvalue (`self.GetOwner`))
  (bind _returnvalue_2 (`|SpawnActorFromClass` (`.SpawnedClass` (break `ItemStruct` EquipInfo)) (`self.GetTransform` _returnvalue) "Undefined" "OverrideRootScale" _returnvalue null))
  (bind _structout (setmembers `ItemStruct` :`StructRef` EquipInfo :`SpawnedActor` _returnvalue_2))
  (`KismetArrayLibrary.Array_Set` (`self.EquipSlots`) (`local.Cursor`) _structout)
  (if (== (`|GetArrayItem` (`self.SocketNames`) (`local.Cursor`)) "None")
    (`self.DisableActor` _returnvalue_2 true)
    (else
      (bind _asbp_player_character (cast `/Game/E4/Blueprints/BP_PlayerCharacter` (`self.GetOwner`)))
      (`self.K2_AttachToComponent` _returnvalue_2 (`Character.Mesh` _asbp_player_character) (`|GetArrayItem` (`self.SocketNames`) (`local.Cursor`)) "SnapToTarget" "SnapToTarget" "SnapToTarget" true))))

(fn `AddNewEquip`
  (params (NewEquip :type "ItemStruct Structure"))
  (returns (IsSucceed :type Boolean))
  (bind (_isempty _equipcursor) (`self.CheckEmptySlot` NewEquip))
  (if _isempty
    (`self.AddEquip` (`local.NewEquip`) _equipcursor)
    (return true)
    (else
      (return false))))

(fn `Check`
  (params (Offset :type Integer) (Num :type Integer))
  (returns (IsEmpty :type Boolean) (EquipCursor :type Integer))
  (for _index (range Offset Num)
    (if (== (`.Name` (break `ItemStruct` (`|GetArrayItem` (`self.EquipSlots`) _index))) "None")
      (return true _index)))
  (return false 0))

(fn `CheckEmptySlot`
  (params (NewEquip :type "ItemStruct Structure"))
  (returns (IsEmpty :type Boolean) (EquipCursor :type Integer))
  (bind (_name _droppedclass _spawnedclass _spawnedactor _canequip _equiptype) (break `ItemStruct` NewEquip))
  (if _canequip
    (switch `EWeaponType` _equiptype
      (:`Weapon`
        (bind (_isempty _equipcursor) (`self.Check` 0 (`self.WeaponNum`)))
        (return _isempty _equipcursor))
      (:`Equip`
        (bind (_isempty_2 _equipcursor_2) (`self.Check` (`self.WeaponNum`) (`self.EquipNum`)))
        (return _isempty_2 _equipcursor_2)))
    (else
      (`KismetSystemLibrary.PrintString` "EquipSlots CheckEmptySlot Error: Can Equip false"))))

(fn `DisableActor`
  (params (SpawnedActor :type "Actor Object Reference") (Disable :type Boolean))
  (bind _returnvalue (not Disable))
  (`self.SetActorHiddenInGame` SpawnedActor Disable)
  (`self.SetActorEnableCollision` SpawnedActor _returnvalue)
  (`self.SetActorTickEnabled` SpawnedActor _returnvalue))

(fn `GetWeaponByCursor`
  (returns (IsSucceed :type Boolean) (WeaponActor :type "Actor Object Reference"))
  (bind (_name _droppedclass _spawnedclass _spawnedactor) (break `ItemStruct` (`|GetArrayItem` (`self.EquipSlots`) (`self.WeaponCursor`))))
  (if (!= _name "None")
    (return true _spawnedactor)
    (else
      (return false null))))

(fn `SetSocketNames`
  (params (CharacterSockets :type "Array of Name"))
  (bind _returnvalue (`KismetArrayLibrary.Array_Length` CharacterSockets))
  (bind _returnvalue_2 (`KismetArrayLibrary.Array_Length` (`self.SocketNames`)))
  (if (== _returnvalue _returnvalue_2)
    _
    (else
      _))
  (for _index (range (`KismetMathLibrary.Min` _returnvalue _returnvalue_2))
    (`KismetArrayLibrary.Array_Set` (`self.SocketNames`) _index (`|GetArrayItem` (`local.CharacterSockets`) _index))))

(fn `SetWeaponCursor`
  (params (Cursor :type Integer))
  (set `self.WeaponCursor` Cursor)
  (bind _asbp_player_character (cast `/Game/E4/Blueprints/BP_PlayerCharacter` (`self.GetOwner`)))
  (`/Game/E4/Blueprints/BP_PlayerCharacter.GetPrimaryWeapon` _asbp_player_character))

(fn `UserConstructionScript`
  (set `self.TotalNum` (+ (`self.WeaponNum`) (`self.EquipNum`)))
  (for _ (range 1 (+ (`self.TotalNum`) 1))
    (`KismetArrayLibrary.Array_Add` (`self.EquipSlots`))
    (`KismetArrayLibrary.Array_Add` (`self.SocketNames`))))