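; Player rifle that fires BP_Projectile with muzzle flash and sound, spending a bullet per shot or playing an empty sound at zero.
; Each tick traces mesh origin to muzzle socket for obstructions, otherwise along the follow camera for the aim point.
; UseItem fires from the socket toward that point, or from the blocking hit toward the socket when obstructed.
; A socket-to-aim trace exists as a placeholder for a future barrel-aim indicator.
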(event `/Game/E4/Blueprints/Interface_PlayerToActor.UseItem`
  (bind _bullets (`self.Bullets`))
  (bind _sm_rifle (`self.SM_Rifle`))
  (bind _linetracehitlocation (`self.LineTraceHitLocation`))
  (bind _ownerpawn (`self.OwnerPawn`))
  (bind _returnvalue (`SceneComponent.GetSocketLocation` _sm_rifle (`self.SocketName`)))
  (if (!= _bullets 0)
    (set `self.Bullets` (- _bullets 1))
    (if (`self.SocketLineHit`)
      (bind _bulletspawntransform (`self.SetBulletDirection` _linetracehitlocation _returnvalue))
      (`|SpawnActorFromClass` "/Game/E4/Blueprints/Weapon/BP_Projectile.BP_Projectile_C" _bulletspawntransform "Undefined" "OverrideRootScale" self _ownerpawn)
      (else
        (bind _bulletspawntransform_2 (`self.SetBulletDirection` _returnvalue _linetracehitlocation))
        (`|SpawnActorFromClass` "/Game/E4/Blueprints/Weapon/BP_Projectile.BP_Projectile_C" _bulletspawntransform_2 "Undefined" "OverrideRootScale" self _ownerpawn)))
    (`GameplayStatics.SpawnEmitterAttached` "/Game/WeaponEffects/P_AssaultRifle_MF.P_AssaultRifle_MF" _sm_rifle "Muzzle" (0.0 0.0 0.0) (struct) (0.5 0.5 0.5))
    (`GameplayStatics.PlaySoundAtLocation` "/Game/E4/Weapon/SM_Rifle/SM_Rifle_sound.SM_Rifle_sound" _returnvalue (struct) 1.0 1.0 0.0 null null null null)
    (else
      (`self.NeedReload`))))

(event `self.ReceiveTick`
  (params (DeltaSeconds :type "Float (single-precision)"))
  (`|ExecutionSequence`
    (:`then_1`
      (bind (_hitlocation _socketlinehit) (`self.LineTraceToSocket`))
      (bind _output_get (set `self.SocketLineHit` _socketlinehit))
      (if _output_get
        (set `self.LineTraceHitLocation` _hitlocation)
        (else
          (bind (_cameralinehit _cameralineend) (`self.LineTraceByCamera`))
          (if (!= _cameralinehit (0.0 0.0 0.0))
            (set `self.LineTraceHitLocation` _cameralinehit)
            (else
              (set `self.LineTraceHitLocation` _cameralineend)
              ;[1 1 1] 나중에 카메라 조준점과 실제 총기 조준점이 일치 하지 않을 경우, 총기 조준점 표시 기능 추가
              (bind _weaponlinehit (`self.LineTraceByWeapon`))
              (if (!= _weaponlinehit (0.0 0.0 0.0))
                _))))))))

(event `self.ReceiveBeginPlay`
  (`self.SetOwnerCamera`)
  (bind `_as폰` (cast `Pawn` (`self.GetOwner`)))
  (set `self.OwnerPawn` `_as폰`))

(fn `GetLineVectByCamera`
  (returns (LineTraceStart :type "Vector Structure") (LineTraceEnd :type "Vector Structure"))
  (bind _ownercamera (`self.OwnerCamera`))
  (bind _returnvalue (`SceneComponent.K2_GetComponentLocation` _ownercamera))
  ;[1 1 1] LineTraceByWeapon/Camera에 사용되는 함수
  (return _returnvalue (+ _returnvalue (* (`KismetMathLibrary.GetForwardVector` (`SceneComponent.K2_GetComponentRotation` _ownercamera)) 5000.0))))

(fn `LineTraceByCamera`
  (returns (CameraLineHit :type "Vector Structure") (CameraLineEnd :type "Vector Structure"))
  (bind (_linetracestart _linetraceend) (`self.GetLineVectByCamera`))
  (bind _outhit (`KismetSystemLibrary.LineTraceSingle` _linetracestart _linetraceend "TraceTypeQuery1"))
  (bind (_bblockinghit _binitialoverlap _time _distance _location _impactpoint _normal _impactnormal _physmat _hitactor _hitcomponent _hitbonename _bonename _hititem _elementindex _faceindex _tracestart _traceend) (`GameplayStatics.BreakHitResult` _outhit))
  (return _location _traceend))

(fn `LineTraceByWeapon`
  (returns (WeaponLineHit :type "Vector Structure") (WeaponLineEnd :type "Vector Structure"))
  (bind (_linetracestart _linetraceend) (`self.GetLineVectByCamera`))
  (bind _outhit (`KismetSystemLibrary.LineTraceSingle` (`SceneComponent.GetSocketLocation` (`self.SM_Rifle`) (`self.SocketName`)) _linetraceend "TraceTypeQuery1"))
  (bind (_bblockinghit _binitialoverlap _time _distance _location _impactpoint _normal _impactnormal _physmat _hitactor _hitcomponent _hitbonename _bonename _hititem _elementindex _faceindex _tracestart _traceend) (`GameplayStatics.BreakHitResult` _outhit))
  (return _location _traceend))

(fn `LineTraceToSocket`
  (returns (HitLocation :type "Vector Structure") (SocketLineHit :type Boolean))
  (bind _sm_rifle (`self.SM_Rifle`))
  (bind _outhit (`KismetSystemLibrary.LineTraceSingle` (`SceneComponent.K2_GetComponentLocation` _sm_rifle) (`SceneComponent.GetSocketLocation` _sm_rifle (`self.SocketName`)) "TraceTypeQuery1" false (`|MakeArray` (`self.GetOwner`))))
  (bind (_bblockinghit _binitialoverlap _time _distance _location) (`GameplayStatics.BreakHitResult` _outhit))
  (return _location (!= _location (0.0 0.0 0.0))))

(fn `NeedReload`
  (`GameplayStatics.PlaySoundAtLocation` "/Game/E4/Weapon/SM_Rifle/NoBullets.NoBullets" (`SceneComponent.K2_GetComponentLocation` (`self.SM_Rifle`)) (struct) 1.0 1.0 0.0 null null null null))

(fn `SetBulletDirection`
  (params (BulletSpawnLocation :type "Vector Structure") (BulletTarget :type "Vector Structure"))
  (returns (BulletSpawnTransform :type "Transform Structure"))
  (return (`KismetMathLibrary.MakeTransform` BulletSpawnLocation (`KismetMathLibrary.Conv_VectorToRotator` (- BulletTarget BulletSpawnLocation)))))

(fn `SetOwnerCamera`
  (bind _asbp_player_character (cast `/Game/E4/Blueprints/BP_PlayerCharacter` (`self.GetOwner`)))
  (set `self.OwnerCamera` (`/Game/E4/Blueprints/BP_PlayerCharacter.FollowCamera` _asbp_player_character)))

(fn `UserConstructionScript`)