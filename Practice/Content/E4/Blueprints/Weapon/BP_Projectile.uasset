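; Weapon projectile that ignores its instigator when moving, trails a particle effect, and deals point damage to what it strikes.
; Overlaps allow penetration: each newly overlapped actor subtracts a physical-material-based value from Energy, and the projectile is destroyed once that runs out.
; Blocking hits deal damage and destroy it immediately.
; Both paths spawn impact particles and sounds looked up by physical material.
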(event `self.ReceiveBeginPlay`
  (`PrimitiveComponent.IgnoreActorWhenMoving` (`self.SphereCollision`) (`self.GetInstigator`) true)
  (`NiagaraFunctionLibrary.SpawnSystemAttached` "/Game/E4/Effects/BulletTrail/EM_BulletTrail.EM_BulletTrail" (`self.SphereMesh`) "BulletTrail" (0.0 0.0 0.0) (struct) "KeepRelativeOffset"))

(event `self.SphereCollision.OnComponentBeginOverlap`
  (params (OverlappedComponent :type "PrimitiveComponent Object Reference") (OtherActor :type "Actor Object Reference") (OtherComp :type "PrimitiveComponent Object Reference") (OtherBodyIndex :type Integer) (bFromSweep :type Boolean) (SweepResult :type "HitResult Structure (by ref)"))
  (if (!= (`self.OverlappedActor`) OtherActor)
    (set `self.OverlappedActor` OtherActor)
    (`self.CalEnergyByImpulse` SweepResult)
    (bind _hitdirection (`self.Hit Effect by Phys Mat` SweepResult))
    (`GameplayStatics.ApplyPointDamage` OtherActor 10.0 _hitdirection SweepResult)
    (if (<= (`self.Energy`) 0.0)
      (`self.K2_DestroyActor`))))

(event `self.SphereCollision.OnComponentHit`
  (params (HitComponent :type "PrimitiveComponent Object Reference") (OtherActor :type "Actor Object Reference") (OtherComp :type "PrimitiveComponent Object Reference") (NormalImpulse :type "Vector Structure") (Hit :type "HitResult Structure (by ref)"))
  (bind _hitdirection (`self.Hit Effect by Phys Mat` Hit))
  (`GameplayStatics.ApplyPointDamage` OtherActor 10.0 _hitdirection Hit)
  (`self.K2_DestroyActor`))

(fn `CalEnergyByImpulse`
  (params (Hit :type "HitResult Structure"))
  (set `self.Energy` (- (`self.Energy`) (`BlueprintMapLibrary.Map_Find` (`self.ImpulseByPhysMat`) (`.PhysMat` (`GameplayStatics.BreakHitResult` Hit))))))

(fn `GetLinePos`
  (params (HitComponent :type "SceneComponent Object Reference"))
  (returns (LineStart :type "Vector Structure") (LineEnd :type "Vector Structure") (DirectRotator :type "Rotator Structure"))
  (bind _returnvalue (`SceneComponent.K2_GetComponentLocation` HitComponent))
  (bind _returnvalue_2 (+ _returnvalue (* (`KismetMathLibrary.GetForwardVector` (`SceneComponent.K2_GetComponentRotation` HitComponent)) 1000.0)))
  (return _returnvalue _returnvalue_2 (`KismetMathLibrary.MakeRotFromZ` (- _returnvalue _returnvalue_2))))

(fn `Hit Effect by Phys Mat`
  (params (Hit :type "HitResult Structure"))
  (returns (HitDirection :type "Vector Structure"))
  (bind (_bblockinghit _binitialoverlap _time _distance _location _impactpoint _normal _impactnormal _physmat _hitactor _hitcomponent _hitbonename _bonename _hititem _elementindex _faceindex _tracestart _traceend) (`GameplayStatics.BreakHitResult` Hit))
  (bind _returnvalue (- _tracestart _traceend))
  (`GameplayStatics.SpawnEmitterAtLocation` (`BlueprintMapLibrary.Map_Find` (`self.ParticleByPhysMat`) _physmat) _location (`KismetMathLibrary.MakeRotFromZ` _returnvalue))
  (`GameplayStatics.PlaySoundAtLocation` (`BlueprintMapLibrary.Map_Find` (`self.ImpactsByPhysMat`) _physmat) _location (struct) 1.0 1.0 0.0 "/Game/E4/Blueprints/TestSoundAttenuation.TestSoundAttenuation" null null null)
  (return _returnvalue))

(fn `UserConstructionScript`)