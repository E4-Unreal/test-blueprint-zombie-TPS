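; BP_Grenade is a thrown grenade weapon that explodes on a timer.
; BeginPlay and UseItem share a DoOnce that enables physics on the Sphere and launches it along the owner's forward vector, so the throw normally fires at BeginPlay.
; A two-second timer then calls Explode, which spawns an explosion effect and sound, applies full radial damage without falloff, and destroys the actor.
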(event `self.ReceiveBeginPlay`
  (bind _sphere (`self.Sphere`))
  (`parent.ReceiveBeginPlay`)
  (`/Engine/EditorBlueprintResources/StandardMacros.DoOnce` false :!label _label
    (:`Completed`
      (`PrimitiveComponent.SetSimulatePhysics` _sphere true)
      (`PrimitiveComponent.SetAllPhysicsLinearVelocity` _sphere (* (`self.GetActorForwardVector` (`self.GetOwner`)) 500.0) false)
      (`KismetSystemLibrary.K2_SetTimer` null "Explode" 2.0))))

(event `/Game/E4/Blueprints/Interface_PlayerToActor.UseItem`
  (goto _label))

(fn `Explode`
  (bind _returnvalue (`self.K2_GetActorLocation`))
  (`GameplayStatics.SpawnEmitterAtLocation` "/Game/StarterContent/Particles/P_Explosion.P_Explosion" _returnvalue (struct) (2.0 2.0 2.0))
  (`GameplayStatics.PlaySoundAtLocation` "/Game/StarterContent/Audio/Explosion01.Explosion01" _returnvalue (struct) 1.0 1.0 0.0 null null null null)
  (`GameplayStatics.ApplyRadialDamage` :`BaseDamage` 100.0 :`Origin` _returnvalue :`DamageRadius` 500.0 :`DamageCauser` self :`InstigatedByController` (`self.GetInstigatorController`) :`bDoFullDamage` true)
  (`self.K2_DestroyActor`))

(fn `UserConstructionScript`
  (`parent.UserConstructionScript`))