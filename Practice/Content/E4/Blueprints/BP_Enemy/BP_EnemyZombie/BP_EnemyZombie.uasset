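; Zombie enemy Blueprint that extends a parent enemy class with movement and melee attack behavior.
; It enters run mode on BeginPlay and switches to walk mode when point damage leaves health at or below half.
; Each attack event alternates between left- and right-hand standing attack montages through a toggle, clearing the attacking flag when the montage completes.
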(event `self.ReceiveBeginPlay`
  (`parent.ReceiveBeginPlay`)
  (`self.SetRunMode`))

(event `self.ReceiveTick`
  (params (DeltaSeconds :type "Float (single-precision)"))
  (`parent.ReceiveTick` DeltaSeconds))

(event `self.ReceivePointDamage`
  (params (Damage :type "Float (single-precision)") (DamageType :type "DamageType Object Reference") (HitLocation :type "Vector Structure") (HitNormal :type "Vector Structure") (HitComponent :type "PrimitiveComponent Object Reference") (BoneName :type Name) (ShotFromDirection :type "Vector Structure") (InstigatedBy :type "Controller Object Reference") (DamageCauser :type "Actor Object Reference") (HitInfo :type "HitResult Structure (by ref)"))
  (`parent.ReceivePointDamage` Damage DamageType HitLocation HitNormal HitComponent BoneName ShotFromDirection InstigatedBy DamageCauser HitInfo)
  (if (<= (/ (`self.Health`) (`self.InitHealth`)) 0.5)
    (`self.SetWalkMode`)))

(event `Attack_Event`
  (bind _mesh (`self.Mesh`))
  (`parent.Attack_Event`)
  (if (`self.HandChange`)
    (set `self.HandChange` false)
    (`|PlayMontage` _mesh "/Game/BSP_ZombieAnims/Animations/Standing/Attack/AS_NAAT_Zombie_Attack_LH_Stand_Montage.AS_NAAT_Zombie_Attack_LH_Stand_Montage"
      (:`OnCompleted`
        _))
    (else
      (set `self.HandChange` true)
      (`|PlayMontage` _mesh "/Game/BSP_ZombieAnims/Animations/Standing/Attack/AS_NAAT_Zombie_Attack_RH_Stand_Montage.AS_NAAT_Zombie_Attack_RH_Stand_Montage"
        (:`OnCompleted`
          _))))
  (set `self.IsAttacking` false))

(fn `SetHealth`
  (params (Damage :type "Float (double-precision)"))
  (`parent.SetHealth` Damage))

(fn `UserConstructionScript`
  (`parent.UserConstructionScript`))