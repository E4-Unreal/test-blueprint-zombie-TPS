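; Enemy character that tracks health, shows it on an HP bar widget and is destroyed when health runs out.
; PointDamage subtracts health, doubling the damage and printing a debug message for hits on the head bone.
; AnyDamage subtracts nothing itself; it refreshes the bar's health percentage and handles death, so only point damage lowers health.
; BeginPlay caches the EnemyHPBar widget from its component and initializes the bar.
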(event `self.ReceiveBeginPlay`
  (bind _asenemy_hpbar (cast `/Game/E4/Blueprints/BP_Enemy/EnemyHPBar` (`WidgetComponent.GetUserWidgetObject` (`self.HP_Bar_Widget`))))
  (set `self.HP_Bar_UI` _asenemy_hpbar)
  (`self.SetHP_Bar`))

(event `self.ReceiveAnyDamage`
  (params (Damage :type "Float (single-precision)") (DamageType :type "DamageType Object Reference") (InstigatedBy :type "Controller Object Reference") (DamageCauser :type "Actor Object Reference"))
  (`self.SetHealth` 0.0)
  (`self.SetHP_Bar`)
  (if (<= (`self.health`) 0.0)
    (`self.K2_DestroyActor`)))

(event `self.ReceivePointDamage`
  (params (Damage :type "Float (single-precision)") (DamageType :type "DamageType Object Reference") (HitLocation :type "Vector Structure") (HitNormal :type "Vector Structure") (HitComponent :type "PrimitiveComponent Object Reference") (BoneName :type Name) (ShotFromDirection :type "Vector Structure") (InstigatedBy :type "Controller Object Reference") (DamageCauser :type "Actor Object Reference") (HitInfo :type "HitResult Structure (by ref)"))
  (bind _final_damage (`self.CalDmgFromBone` BoneName Damage))
  (`self.SetHealth` _final_damage))

(fn `CalDmgFromBone`
  (params (bone :type Name) (damage :type "Float (double-precision)"))
  (returns (final_damage :type "Float (double-precision)"))
  (if (== bone "head")
    (`KismetSystemLibrary.PrintString` "HeadShot")
    (return (* damage 2.0))
    (else
      (return damage))))

(fn `SetHealth`
  (params (damage :type "Float (double-precision)"))
  (set `self.health` (- (`self.health`) damage)))

(fn `SetHP_Bar`
  (set `/Game/E4/Blueprints/BP_Enemy/EnemyHPBar.HP_Percent` (/ (`self.health`) (`self.init_health`)) (`self.HP_Bar_UI`)))

(fn `UserConstructionScript`)