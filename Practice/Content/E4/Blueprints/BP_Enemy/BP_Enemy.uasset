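; BP_Enemy is an enemy actor that takes damage and shows its remaining health on a widget-component HP bar.
; On BeginPlay it casts the HPBarWidget's user widget to EnemyHPBar, stores it and sets the initial fill ratio from Health over InitHealth.
; AnyDamage subtracts the damage, updates the bar's percent and destroys the actor when health reaches zero or below.
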(event `self.ReceiveBeginPlay`
  (bind _asenemy_hpbar (cast `/Game/E4/Blueprints/BP_Enemy/EnemyHPBar` (`WidgetComponent.GetUserWidgetObject` (`self.HPBarWidget`))))
  (bind _output_get (set `self.HP_Bar_UI` _asenemy_hpbar))
  (set `/Game/E4/Blueprints/BP_Enemy/EnemyHPBar.HP_Percent` (/ (`self.health`) (`self.init_health`)) _output_get))

(event `self.ReceiveAnyDamage`
  (params (Damage :type "Float (single-precision)") (DamageType :type "DamageType Object Reference") (InstigatedBy :type "Controller Object Reference") (DamageCauser :type "Actor Object Reference"))
  (set `self.health` (- (`self.health`) Damage))
  (set `/Game/E4/Blueprints/BP_Enemy/EnemyHPBar.HP_Percent` (/ (`self.health`) (`self.init_health`)) (`self.HP_Bar_UI`))
  (if (<= (`self.health`) 0.0)
    (`self.K2_DestroyActor`)))

(fn `UserConstructionScript`)