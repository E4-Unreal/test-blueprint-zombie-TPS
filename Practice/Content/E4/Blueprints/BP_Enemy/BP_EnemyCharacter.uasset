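; BP_EnemyCharacter is a damageable enemy character with a health bar widget, extending a parent class that supplies health, bone-based damage and death logic.
; The bar starts hidden and caches its UI on BeginPlay, along with the AI controller.
; Point damage is scaled by hit bone through the parent, then updates health and reveals the bar.
; At zero health it runs parent death, hides the bar and expires the AI controller almost instantly.
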(event `self.ReceiveBeginPlay`
  (`parent.ReceiveBeginPlay`)
  (`self.InitHP_Bar`)
  (set `self.AIController` (`AIBlueprintHelperLibrary.GetAIController` self)))

(event `self.ReceiveActorBeginOverlap`
  (params (OtherActor :type "Actor Object Reference"))
  (`parent.ReceiveActorBeginOverlap` OtherActor))

(event `self.ReceiveTick`
  (params (DeltaSeconds :type "Float (single-precision)"))
  (`parent.ReceiveTick` DeltaSeconds))

(event `self.ReceiveAnyDamage`
  (params (Damage :type "Float (single-precision)") (DamageType :type "DamageType Object Reference") (InstigatedBy :type "Controller Object Reference") (DamageCauser :type "Actor Object Reference"))
  (`parent.ReceiveAnyDamage` Damage DamageType InstigatedBy DamageCauser))

(event `self.ReceivePointDamage`
  (params (Damage :type "Float (single-precision)") (DamageType :type "DamageType Object Reference") (HitLocation :type "Vector Structure") (HitNormal :type "Vector Structure") (HitComponent :type "PrimitiveComponent Object Reference") (BoneName :type Name) (ShotFromDirection :type "Vector Structure") (InstigatedBy :type "Controller Object Reference") (DamageCauser :type "Actor Object Reference") (HitInfo :type "HitResult Structure (by ref)"))
  (`parent.ReceivePointDamage` Damage DamageType HitLocation HitNormal HitComponent BoneName ShotFromDirection InstigatedBy DamageCauser HitInfo)
  (bind _calculateddamage (`self.CalDmgByBone` BoneName Damage))
  (`self.SetHealth` _calculateddamage)
  (`self.SetHP_Bar`)
  (if (<= (`self.Health`) 0.0)
    (`self.SetDead`)
    (else
      (`SceneComponent.SetHiddenInGame` (`self.HP_Bar_Widget`) false false))))

(fn `CalDmgByBone`
  (params (BoneName :type Name) (Damage :type "Float (double-precision)"))
  (returns (CalculatedDamage :type "Float (double-precision)"))
  (bind _calculateddamage (`parent.CalDmgByBone` BoneName Damage))
  (return _calculateddamage))

(fn `InitHP_Bar`
  (bind _asenemy_hpbar (cast `/Game/E4/Blueprints/BP_Enemy/EnemyHPBar` (`WidgetComponent.GetUserWidgetObject` (`self.HP_Bar_Widget`))))
  (set `self.HP_Bar_UI` _asenemy_hpbar)
  (`self.SetHP_Bar`)
  (`SceneComponent.SetHiddenInGame` (`self.HP_Bar_Widget`) true false))

(fn `SetDead`
  (`parent.SetDead`)
  (`self.SetLifeSpan` (`self.AIController`) 0.0001)
  (`SceneComponent.SetHiddenInGame` (`self.HP_Bar_Widget`) true false))

(fn `SetHealth`
  (params (Damage :type "Float (double-precision)"))
  (`parent.SetHealth` Damage))

(fn `SetHP_Bar`
  (set `/Game/E4/Blueprints/BP_Enemy/EnemyHPBar.HP_Percent` (/ (`self.Health`) (`self.InitHealth`)) (`self.HP_Bar_UI`)))

(fn `UserConstructionScript`)