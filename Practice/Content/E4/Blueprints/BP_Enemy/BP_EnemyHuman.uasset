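; BP_EnemyHuman is a human enemy Blueprint that extends its parent with a directional hit reaction and sets a fixed walk speed on BeginPlay.
; On point damage, it runs the parent logic, then takes the yaw difference between the capsule's rotation and the shot direction.
; That yaw is classed as "Front" or "Back", which keys a map lookup for the hit montage played on the mesh.
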(event `self.ReceiveBeginPlay`
  (`parent.ReceiveBeginPlay`)
  (set `CharacterMovementComponent.MaxWalkSpeed` 100.0 (`self.CharacterMovement`)))

(event `self.ReceivePointDamage`
  (params (Damage :type "Float (single-precision)") (DamageType :type "DamageType Object Reference") (HitLocation :type "Vector Structure") (HitNormal :type "Vector Structure") (HitComponent :type "PrimitiveComponent Object Reference") (BoneName :type Name) (ShotFromDirection :type "Vector Structure") (InstigatedBy :type "Controller Object Reference") (DamageCauser :type "Actor Object Reference") (HitInfo :type "HitResult Structure (by ref)"))
  (`parent.ReceivePointDamage` Damage DamageType HitLocation HitNormal HitComponent BoneName ShotFromDirection InstigatedBy DamageCauser HitInfo)
  (bind _relativerotator (`self.CalRelativeRotator_0` ShotFromDirection))
  (bind _direction (`self.GetDirectionByRotator` _relativerotator))
  (`|PlayMontage` (`self.Mesh`) (`BlueprintMapLibrary.Map_Find` (`self.HitAnimByName`) _direction)))

(fn `CalRelativeRotator_0`
  (params (HitDirection :type "Vector Structure"))
  (returns (RelativeRotator :type "Rotator Structure"))
  (return (`KismetMathLibrary.NormalizedDeltaRotator` (`SceneComponent.K2_GetComponentRotation` (`self.CapsuleComponent`)) (`KismetMathLibrary.Conv_VectorToRotator` HitDirection))))

(fn `GetDirectionByRotator`
  (params (RelativeRotator :type "Rotator Structure"))
  (returns (Direction :type Name))
  (bind _yaw (.yaw RelativeRotator))
  (if (and (>= _yaw -90.0) (<= _yaw 90.0))
    (return "Front")
    (else
      (return "Back"))))

(fn `UserConstructionScript`
  (`parent.UserConstructionScript`))