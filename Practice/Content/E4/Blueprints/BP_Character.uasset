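; Character Blueprint that handles health, walk and run speeds, an attacking flag and death.
; Point damage is scaled by a per-bone multiplier map, falling back to raw damage for unlisted bones, then subtracted from Health.
; At zero health it disables damage, destroys the capsule, makes the mesh block pawns and starts ragdoll physics after a short timer.
; A raised mass scale temporarily keeps corpses from rolling too lightly until the physics asset is fixed.
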(event `self.ReceiveBeginPlay`
  (set `self.Health` (`self.InitHealth`))
  (set `CharacterMovementComponent.MaxWalkSpeed` (`self.WalkSpeed`) (`self.CharacterMovement`)))

(event `Attack_Event`
  (set `self.IsAttacking` true))

(event `self.ReceivePointDamage`
  (params (Damage :type "Float (single-precision)") (DamageType :type "DamageType Object Reference") (HitLocation :type "Vector Structure") (HitNormal :type "Vector Structure") (HitComponent :type "PrimitiveComponent Object Reference") (BoneName :type Name) (ShotFromDirection :type "Vector Structure") (InstigatedBy :type "Controller Object Reference") (DamageCauser :type "Actor Object Reference") (HitInfo :type "HitResult Structure (by ref)"))
  (bind _calculateddamage (`self.CalDmgByBone` BoneName Damage))
  (`self.SetHealth` _calculateddamage)
  (if (<= (`self.Health`) 0.0)
    (`self.SetDead`)))

(fn `AfterDeath`
  ;[1 1 1] Set All mass Scale은 시체가 너무 가볍게 굴러다니는 걸 방지하기 위함이자 임시 조치.
  ; 나중에 피직스 에셋 건드려야함
  (`PrimitiveComponent.SetSimulatePhysics` (`self.Mesh`) true))

(fn `CalDmgByBone`
  (params (BoneName :type Name) (Damage :type "Float (double-precision)"))
  (returns (CalculatedDamage :type "Float (double-precision)"))
  (bind (_value _returnvalue) (`BlueprintMapLibrary.Map_Find` (`self.PointDamageByBone`) BoneName))
  (if _returnvalue
    (return (* Damage _value))
    (else
      (return Damage))))

(fn `SetDead`
  (bind _mesh (`self.Mesh`))
  (set `self.IsDead` true)
  (set `self.bCanBeDamaged` false)
  (`ActorComponent.K2_DestroyComponent` (`self.CapsuleComponent`))
  (`PrimitiveComponent.SetCollisionObjectType` _mesh "ECC_WorldDynamic")
  (`PrimitiveComponent.SetCollisionResponseToChannel` _mesh "ECC_Pawn" "ECR_Block")
  (`PrimitiveComponent.SetAllMassScale` _mesh 100.0)
  (`KismetSystemLibrary.K2_SetTimer` null "AfterDeath" 1.5))

(fn `SetHealth`
  (params (Damage :type "Float (double-precision)"))
  (set `self.health` (- (`self.Health`) Damage)))

(fn `SetRunMode`
  (set `CharacterMovementComponent.MaxWalkSpeed` (`self.RunSpeed`) (`self.CharacterMovement`)))

(fn `SetWalkMode`
  (set `CharacterMovementComponent.MaxWalkSpeed` (`self.WalkSpeed`) (`self.CharacterMovement`)))

(fn `UserConstructionScript`)